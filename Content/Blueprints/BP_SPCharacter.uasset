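; BP_SPCharacter is a player character Blueprint that drives the HUD through the in-game and post-game phases.
; On BeginPlay it creates a Main_HUD widget, shows the in-game page through a widget switcher and sets game-only input.
; Weapon change events notify the in-game widget of a pickup.
; On death it switches to the post-game page, triggers the death score, shows the cursor and sets UI-only input.
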(event EventBeginPlay
  (bind _returnvalue (UserInterface|CreateWidget "/Game/UI/Main_HUD.Main_HUD_C"))
  (bind _output_get (Variables|Default|SetUI _returnvalue))
  (Class|WidgetSwitcher|SetActiveWidget (Variables|/Game/UI/Main_HUD.Main_HUD_C|GetWidgetSwitcher_39 _output_get) (Variables|/Game/UI/Main_HUD.Main_HUD_C|GetInGame_Widget _output_get))
  (UserInterface|Viewport|AddtoViewport _output_get 0)
  (Input|SetInputModeGameOnly (Game|GetPlayerController 0)))

(event EventOnDeath
  (bind _returnvalue (Game|GetPlayerController 0))
  (bind _ui (Variables|Default|GetUI))
  (bind _postgame_widget (Variables|/Game/UI/Main_HUD.Main_HUD_C|GetPostGame_Widget _ui))
  (Class|WidgetSwitcher|SetActiveWidget (Variables|/Game/UI/Main_HUD.Main_HUD_C|GetWidgetSwitcher_39 _ui) _postgame_widget)
  (Default|DeathScore _postgame_widget)
  (Variables|/Script/Engine.PlayerController|SetbShowMouseCursor _returnvalue true)
  (Input|SetInputModeUIOnly _returnvalue 0 "DoNotLock"))

(event EventOnWeaponChanged
  (Default|OnWeaponPickUp (Variables|/Game/UI/Main_HUD.Main_HUD_C|GetInGame_Widget (Variables|Default|GetUI))))

(fn ConstructionScript)